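; BP_CraftingTable is a crafting table that holds items and checks whether they combine.
; AddItem appends to the Items array until MaximumItems is reached, reporting whether the item was accepted.
; AttemptCraft runs only on a full table, matching the first item's name against the second item's CompatibleItems.
; A match returns a fixed Axe as ReturnItem but still reports Success as false, like every other path.
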(event EventBeginPlay)

(event Collision|EventActorBeginOverlap
  (params (OtherActor :type Actor%20Object%20Reference)))

(event EventTick
  (params (DeltaSeconds :type Float%20%28single-precision%29)))

(fn ConstructionScript)

(fn AddItem
  (params (Item :type Item%20Data%20Structure))
  (if (== (Utilities|Array|Length (Variables|Default|GetItems)) (Variables|Default|GetMaximumItems))
    (return false)
    (else
      (Utilities|Array|Add (Variables|Default|GetItems) Item)
      (return true))))

(fn AttemptCraft
  (if (== (Utilities|Array|Length (Variables|Default|GetItems)) (Variables|Default|GetMaximumItems))
    (for _array_element (.compatibleitems (Utilities|Array|Get(acopy) (Variables|Default|GetItems) 1))
      (if (Utilities|Enum|Equal(Enum) _array_element (.name (Utilities|Array|Get(acopy) (Variables|Default|GetItems))))
        (return false (Variables|Default|GetAxe))))
    (return false "")
    (else
      (return false ""))))